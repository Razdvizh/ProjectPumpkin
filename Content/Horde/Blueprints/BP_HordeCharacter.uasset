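; BP_HordeCharacter is a horde character that launches itself when it collides with the top-down character.
; It binds to its own actor hit event on BeginPlay and filters hits by casting to BP_TopDownCharacter.
; A suggested arc velocity toward a point PushbackDistance along its forward vector feeds LaunchCharacter, overriding both XY and Z velocity.
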(event Custom|OnActorHit_Event
  (params (SelfActor :type Actor%20Object%20Reference) (OtherActor :type Actor%20Object%20Reference) (NormalImpulse :type Vector) (Hit :type Hit%20Result%20Structure%20%28by%20ref%29))
  (bind _returnvalue (Transformation|GetActorLocation))
  (Utilities|Casting|CastToBP_TopDownCharacter OtherActor)
  (bind _outlaunchvelocity (Game|SuggestProjectileVelocityCustomArc _returnvalue (+ _returnvalue (* (Math|Vector|GetForwardVector (Transformation|GetActorRotation)) (Variables|Default|GetPushback%20distance))) 0.0 0.5))
  (Character|LaunchCharacter _outlaunchvelocity true true))

(event EventBeginPlay
  (Collision|AssignOnActorHit (delegate Custom|OnActorHit_Event)))

(fn ConstructionScript)